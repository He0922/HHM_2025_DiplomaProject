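; BP_MyCharacter is a character Blueprint that, as shown, mainly provides on-screen debugging of its locomotion state.
; Every Tick calls DebugENum, which prints the movement state, gait, movement position and rotation mode enums.
; GetFutureVelocity linearly extrapolates velocity from the movement component's current acceleration over a given time.
; An unconnected print chain for gait, rotation mode and walk/strafe input flags never runs.
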(event `self.ReceiveTick`
  (params (DeltaSeconds :type "Float (single-precision)"))
  (`KismetSystemLibrary.PrintString` " \n \n \n \n \n \n \n \n \n" true true (struct :`G` 0.66 :`B` 1.0 :`A` 1.0) 0.0)
  (`self.DebugENum`))

(fn `DebugENum`
  (`KismetSystemLibrary.PrintString` (`KismetStringLibrary.Concat_StrStr` "Character Movement State: " (`|GetEnumeratorNameAsString` (`self.MovementState`))) true true (struct :`G` 0.66 :`B` 1.0 :`A` 1.0) 0.0)
  (`KismetSystemLibrary.PrintString` (`KismetStringLibrary.Concat_StrStr` "Character Gait: " (`|GetEnumeratorNameAsString` (`self.Gait`))) true true (struct :`G` 0.66 :`B` 1.0 :`A` 1.0) 0.0)
  (`KismetSystemLibrary.PrintString` (`KismetStringLibrary.Concat_StrStr` "Character Movement Position:  " (`|GetEnumeratorNameAsString` (`self.MovementPosition`))) true true (struct :`G` 0.66 :`B` 1.0 :`A` 1.0) 0.0)
  (`KismetSystemLibrary.PrintString` (`KismetStringLibrary.Concat_StrStr` "Character Rotation Mode: " (`|GetEnumeratorNameAsString` (`self.RotationMode`))) true true (struct :`G` 0.66 :`B` 1.0 :`A` 1.0) 0.0))

(fn `GetFutureVelocity`
  (params (FutureTime :type "Float (double-precision)"))
  (returns (ReturnValue :type "Vector Structure"))
  (return (+ (`self.GetVelocity`) (* (`CharacterMovementComponent.GetCurrentAcceleration` (`self.MovementComponent`)) (`local.FutureTime`)))))

(fn `UserConstructionScript`)