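; Player character Blueprint that drives controller-based rotation and prints locomotion debug info every frame.
; Tick prints the just-landed flag and calls DebugEnum to print gait, rotation mode, movement state and movement mode.
; When orient-to-movement is off, Tick enables controller desired rotation while moving and disables it while idle.
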(event `self.ReceiveBeginPlay`)

(event `self.ReceiveTick`
  (params (DeltaSeconds :type "Float (single-precision)"))
  (`KismetSystemLibrary.PrintString` " \n \n \n" true true (struct :`G` 0.66 :`B` 1.0 :`A` 1.0) 0.0)
  (`self.DebugEnum`)
  (`KismetSystemLibrary.PrintString` (`KismetStringLibrary.Concat_StrStr` "Justed Landed: " (`KismetStringLibrary.Conv_BoolToString` (`self.bJustedLanded`))) true true (struct :`G` 0.66 :`B` 1.0 :`A` 1.0) 0.0)
  (if (not (`CharacterMovementComponent.bOrientRotationToMovement` (`self.MovementComponent`)))
    (switch `EMovementStates` (`self.MovementStates`)
      (:`Idle`
        (set `CharacterMovementComponent.bUseControllerDesiredRotation` false (`self.MovementComponent`)))
      (:`Moving`
        (set `CharacterMovementComponent.bUseControllerDesiredRotation` true (`self.MovementComponent`))))))

(fn `DebugEnum`
  (`KismetSystemLibrary.PrintString` (`KismetStringLibrary.Concat_StrStr` "Character Gait: " (`|GetEnumeratorNameAsString` (`self.Gait`))) true true (struct :`G` 0.66 :`B` 1.0 :`A` 1.0) 0.0)
  (`KismetSystemLibrary.PrintString` (`KismetStringLibrary.Concat_StrStr` "Character RotationMode: " (`|GetEnumeratorNameAsString` (`self.RotationMode`))) true true (struct :`G` 0.66 :`B` 1.0 :`A` 1.0) 0.0)
  (`KismetSystemLibrary.PrintString` (`KismetStringLibrary.Concat_StrStr` "Character Movement States: " (`|GetEnumeratorNameAsString` (`self.MovementStates`))) true true (struct :`G` 0.66 :`B` 1.0 :`A` 1.0) 0.0)
  (`KismetSystemLibrary.PrintString` (`KismetStringLibrary.Concat_StrStr` "Character Movement Position: " (`|GetEnumeratorNameAsString` (`self.MovementMode`))) true true (struct :`G` 0.66 :`B` 1.0 :`A` 1.0) 0.0))

(fn `UserConstructionScript`)